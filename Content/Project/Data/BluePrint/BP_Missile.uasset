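; BP_Missile is a missile Blueprint that fires a physics-driven Rocket when the Space Bar is pressed, also printing a debug string.
; DoShot moves the Rocket to the location and rotation of MainActor's root, clears its linear velocity, then applies a large forward impulse.
; The same Rocket is repositioned and relaunched on each shot, with no new projectile spawned.
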(event `self.ReceiveBeginPlay`)

(event `Key|SpaceBar`
  (params (Key :type "Key Structure"))
  (:`Pressed`
    (`self.DoShot`)
    (`KismetSystemLibrary.PrintString` "Hello")))

(fn `DoShot`
  (bind _mainactor (`self.MainActor`))
  (bind _rocket (`self.Rocket`))
  (`SceneComponent.K2_SetWorldLocationAndRotation` (`self.Rocket`) (`SceneComponent.K2_GetComponentLocation` (`Actor.RootComponent` _mainactor)) (`SceneComponent.K2_GetComponentRotation` (`Actor.RootComponent` _mainactor)) false false)
  (`PrimitiveComponent.SetAllPhysicsLinearVelocity` _rocket (0.0 0.0 0.0) false)
  (`PrimitiveComponent.AddImpulse` _rocket (* (`SceneComponent.GetForwardVector` _rocket) 300000.0) "None" false))

(fn `UserConstructionScript`)